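; BP_FadeActor is a mesh actor that can fade out and back in through FadeOut and Fadein events.
; At BeginPlay it builds M_FadeObject dynamic instances, copying base color, normal and ORM textures from the materials saved at construction.
; FadeOut swaps these in, ignores Visibility and GameTraceChannel2 collision, and drives their Fade parameter by timeline.
; Fadein restores the collision profile and reverses the timeline, restoring original materials when Fade finishes at 1.
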(event `self.ReceiveBeginPlay`
  (set `self.OriginalCollisionProfile` (`PrimitiveComponent.GetCollisionProfileName` (`self.Mesh`)))
  (`KismetArrayLibrary.Array_Clear` (`self.DynamicMaterialInstances`))
  (for (_ _array_index) (`self.OriginalMaterials`)
    (bind _returnvalue (`KismetMaterialLibrary.CreateDynamicMaterialInstance` "/Game/Blueprints/Actor/FadeActor/M_FadeObject.M_FadeObject"))
    (`KismetArrayLibrary.Array_Add` (`self.DynamicMaterialInstances`) _returnvalue)
    (for _array_element (`|MakeArray` "BaseColorTexture" "NormalTexture" "ORMTexture")
      (bind _asmaterial_instance_constant (cast `MaterialInstanceConstant` (`|GetArrayItem` (`self.OriginalMaterials`) _array_index)))
      (bind _returnvalue_2 (`MaterialInstanceConstant.K2_GetTextureParameterValue` _asmaterial_instance_constant _array_element))
      (`MaterialInstanceDynamic.SetTextureParameterValue` _returnvalue _array_element _returnvalue_2))))

(event `/Game/Blueprints/Actor/FadeActor/BI_FadeInterface.FadeOut`
  (`self.DisableCollisionResponses`)
  (`self.UpdateMaterials` (`self.DynamicMaterialInstances`))
  (bind (_direction _fade) (`Timeline|FadeTimeline` :!label _label)
    (:`Update`
      (for _array_element (`self.DynamicMaterialInstances`)
        (`MaterialInstanceDynamic.SetScalarParameterValue` _array_element "Fade" _fade)))
    (:`Finished`
      (`self.OnFadeFinished` _fade))))

(event `/Game/Blueprints/Actor/FadeActor/BI_FadeInterface.FadeIn`
  (`self.ResetCollisionProfile`)
  (goto _label :!via `Reverse`))

(fn `DisableCollisionResponses`
  (bind _mesh (`self.Mesh`))
  (`PrimitiveComponent.SetCollisionResponseToChannel` _mesh "ECC_Visibility" "ECR_Ignore")
  (`PrimitiveComponent.SetCollisionResponseToChannel` _mesh "ECC_GameTraceChannel2" "ECR_Ignore"))

(fn `OnFadeFinished`
  (params (Fade :type "Float (double-precision)"))
  (if (>= Fade 1.0)
    (`self.UpdateMaterials` (`self.OriginalMaterials`))))

(fn `ResetCollisionProfile`
  (`PrimitiveComponent.SetCollisionProfileName` (`self.Mesh`) (`self.OriginalCollisionProfile`) true))

(fn `UpdateMaterials`
  (params (Materials :type "Array of MaterialInterface Object Reference"))
  (for (_array_element _array_index) Materials
    (`PrimitiveComponent.SetMaterial` (`self.Mesh`) _array_index _array_element)))

(fn `UserConstructionScript`
  (for _array_element (`MeshComponent.GetMaterials` (`self.Mesh`))
    (`KismetArrayLibrary.Array_Add` (`self.OriginalMaterials`) _array_element)))