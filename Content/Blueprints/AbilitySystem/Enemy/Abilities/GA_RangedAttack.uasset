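; GA_RangedAttack is an enemy gameplay ability that fires a projectile at the avatar's current combat target, ending early if that target is dead.
; It faces the avatar toward the target, then plays a random tagged attack montage.
; A gameplay event matching the montage's tag triggers the projectile spawn from that montage's socket tag, with optional pitch override.
; The ability ends when the montage completes, is interrupted or is cancelled.
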(event `self.K2_ActivateAbility`
  (bind _returnvalue (`self.GetAvatarActorFromActorInfo`))
  (bind (_montage _montagetag _sockettag) (break `TaggedMontage` (`self.TaggedMontage`)))
  (bind _returnvalue_2 (message `EnemyInterface.GetCombatTarget` _returnvalue))
  (bind _returnvalue_3 (message `CombatInterface.IsDead` _returnvalue_2))
  (if _returnvalue_3
    (`self.K2_EndAbility`)
    (else
      (set `self.CombatTarget` _returnvalue_2)
      (bind _ascombat_interface (cast `CombatInterface` _returnvalue))
      (`CombatInterface.UpdateFacingTarget` _ascombat_interface (`Actor.K2_GetActorLocation` (`self.CombatTarget`)))
      (bind _returnvalue_4 (message `CombatInterface.GetAttackMontages` (`self.GetAvatarActorFromActorInfo`)))
      (set `self.TaggedMontage` (`self.GetRandomTaggedMontageFromArray` _returnvalue_4))
      (`AbilityTask_PlayMontageAndWait.CreatePlayMontageAndWaitProxy` "None" _montage 1.0 "None" false
        (:`then`
          (`AbilityTask_WaitGameplayEvent.WaitGameplayEvent` _montagetag null true
            (:`EventReceived`
              (`self.SpawnProjectile` (`Actor.K2_GetActorLocation` (`self.CombatTarget`)) _sockettag (`self.ShouldOverridePitch`) (`self.PitchOverride`)))))
        (:`OnCompleted`
          (`self.K2_EndAbility` :!label _label))
        (:`OnInterrupted`
          (goto _label))
        (:`OnCancelled`
          (goto _label))))))