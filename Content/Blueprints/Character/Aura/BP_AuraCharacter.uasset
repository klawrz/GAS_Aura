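; BP_AuraCharacter is the Aura character Blueprint, handling attack-agnostic facing through motion warping and fading of actors that overlap its Box component.
; UpdateFacingTarget writes the given location to the FacingTarget warp target.
; Box begin and end overlaps send fade-out and fade-in messages through BI_FadeInterface.
; ShouldFade gates both on local control, interface support and nonzero velocity, so an overlap ending while stationary sends no fade-in.
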(event `CombatInterface.UpdateFacingTarget`
  (params (Target :type "Vector Structure (by ref)"))
  (`MotionWarpingComponent.AddOrUpdateWarpTargetFromLocation` (`self.MotionWarping`) "FacingTarget" Target))

(event `self.Box.OnComponentBeginOverlap`
  (params (OverlappedComponent :type "PrimitiveComponent Object Reference") (OtherActor :type "Actor Object Reference") (OtherComp :type "PrimitiveComponent Object Reference") (OtherBodyIndex :type Integer) (bFromSweep :type Boolean) (SweepResult :type "HitResult Structure (by ref)"))
  (bind _shouldfade (`self.ShouldFade` OtherActor))
  (if _shouldfade
    (message `/Game/Blueprints/Actor/FadeActor/BI_FadeInterface.FadeOut` OtherActor)))

(event `self.Box.OnComponentEndOverlap`
  (params (OverlappedComponent :type "PrimitiveComponent Object Reference") (OtherActor :type "Actor Object Reference") (OtherComp :type "PrimitiveComponent Object Reference") (OtherBodyIndex :type Integer))
  (bind _shouldfade (`self.ShouldFade` OtherActor))
  (if _shouldfade
    (message `/Game/Blueprints/Actor/FadeActor/BI_FadeInterface.FadeIn` OtherActor)))

(fn `ShouldFade`
  (params (OtherActor :type "Object Object Reference"))
  (returns (ShouldFade :type Boolean))
  (return (and (`self.IsLocallyControlled`) (`KismetSystemLibrary.DoesImplementInterface` OtherActor "/Game/Blueprints/Actor/FadeActor/BI_FadeInterface.BI_FadeInterface_C") (> (`KismetMathLibrary.VSize` (`MovementComponent.Velocity` (`self.CharacterMovement`))) 0.0))))

(fn `UserConstructionScript`)